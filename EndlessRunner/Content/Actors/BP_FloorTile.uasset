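; BP_FloorTile is a track segment that populates itself with random content and removes itself once the player passes, as in an endless runner.
; Its construction script rolls ObstacleChance to add either one obstacle or several pickups as child actors, with random classes and positions within spawn boxes.
; When the player leaves EndTrigger, it fires Exited and destroys itself after a short delay.
; GetAttachTransform exposes the AttachPoint world transform.
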(event OnComponentEndOverlap(EndTrigger)
  (params (OverlappedComponent :type Primitive%20Component%20Object%20Reference) (OtherActor :type Actor%20Object%20Reference) (OtherComp :type Primitive%20Component%20Object%20Reference) (OtherBodyIndex :type Integer))
  (if (== OtherActor (Game|Player|GetPlayerPawn 0))
    (Default|CallExited self)
    (Utilities|FlowControl|Delay 0.2)
    (Actor|DestroyActor)))

(fn ConstructionScript
  (if (Math|Random|RandomBoolwithWeight (Variables|Default|GetObstacleChance))
    (CallFunction|SpawnObstacle)
    (else
      (CallFunction|SpawnItem))))

(fn GetAttachTransform
  (return (Transformation|GetWorldTransform (Variables|Default|GetAttachPoint))))

(fn SpawnObstacle
  (bind _returnvalue (AddComponent|AddChildActorComponent false (Math|Conversions|ToTransform(Vector) (Math|Random|RandomPointinBoundingBox "0, 0, 0" (Components|Box|GetScaledBoxExtent (Variables|Default|GetObstacleSpawn))))))
  (ChildActorComponent|SetChildActorClass _returnvalue (.OutItem (Utilities|Array|Random (Variables|Default|GetObstacleType)))))

(fn SpawnItem
  (bind _pickupspawn (Variables|Default|GetPickUpSpawn))
  (for _index (range 0 3)
    (bind _returnvalue (AddComponent|AddChildActorComponent false (Math|Conversions|ToTransform(Vector) (Math|Random|RandomPointinBoundingBox (Variables|/Script/Engine.SceneComponent|GetRelativeLocation _pickupspawn) (Components|Box|GetScaledBoxExtent _pickupspawn)))))
    (ChildActorComponent|SetChildActorClass _returnvalue (.OutItem (Utilities|Array|Random (Variables|Default|GetPickUpType))))))